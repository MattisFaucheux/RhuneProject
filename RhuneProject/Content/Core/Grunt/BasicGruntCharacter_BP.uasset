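; Dwarf grunt character that fights for a camp, with body and equipment materials set at BeginPlay from its camp and aura type (Occulte or Celeste).
; Sphere detection overlaps track the closest opposing grunt or player character and raise enemy detected or no-enemy calls.
; Hammer overlaps deal damage while attacking, and incoming damage routes to TakeDamages.
; When enabled, a widget health bar shows within range of the player, yawing toward the camera each tick.
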(event OnComponentBeginOverlap(HammerCollision)
  (params (OverlappedComponent :type Primitive%20Component%20Object%20Reference) (OtherActor :type Actor%20Object%20Reference) (OtherComp :type Primitive%20Component%20Object%20Reference) (OtherBodyIndex :type Integer) (bFromSweep :type Boolean) (SweepResult :type Hit%20Result%20Structure%20%28by%20ref%29))
  (if (Variables|Default|GetIsAttacking)
    (Class|BasicGruntCharacter|DoDamages OtherActor)))

(event OnComponentBeginOverlap(SphereDetection)
  (params (OverlappedComponent :type Primitive%20Component%20Object%20Reference) (OtherActor :type Actor%20Object%20Reference) (OtherComp :type Primitive%20Component%20Object%20Reference) (OtherBodyIndex :type Integer) (bFromSweep :type Boolean) (SweepResult :type Hit%20Result%20Structure%20%28by%20ref%29))
  (bind _spheredetection (Variables|Default|GetSphereDetection))
  (bind _overlappingactors (Collision|GetOverlappingActors _spheredetection 0 :!class /Script/Engine.PrimitiveComponent))
  (if (== (Utilities|Array|Length _overlappingactors) 0)
    (Default|CallOnNoEnemyDetected)
    (else
      (for _array_element _overlappingactors
        (bind _asbasic_grunt_character_bp (Utilities|Casting|CastToBasicGruntCharacter_BP _array_element)
          (:then
            (bind _returnvalue (Class|BasicGruntCharacter|IsSameCamp _asbasic_grunt_character_bp (Variables|Default|GetGruntCamp)))
            (if (not _returnvalue)
              (Utilities|IsValid (Variables|Default|GetClosest%20Actor) :!label _label
                (:Is%20Valid
                  (if (> (Transformation|GetDistanceTo (Variables|Default|GetClosest%20Actor)) (Transformation|GetDistanceTo _array_element))
                    (Variables|Default|SetDistance%20ClosestActor (Transformation|GetDistanceTo (Variables|Default|GetClosest%20Actor)))
                    (Variables|Default|SetClosest%20Actor _array_element)
                    (Default|CallOnEnnemyDetected (Variables|Default|GetClosest%20Actor) (Variables|Default|GetDistance%20ClosestActor) :!label _label_2)
                    (else
                      (Variables|Default|SetDistance%20ClosestActor (Transformation|GetDistanceTo _array_element)))))
                (:Is%20Not%20Valid
                  (Variables|Default|SetDistance%20ClosestActor (Transformation|GetDistanceTo _array_element))
                  (Variables|Default|SetClosest%20Actor _array_element)
                  (goto _label_2)))))
          (:CastFailed
            (Utilities|Casting|CastToRhuneProjectCharacter _array_element)
            (bind _returnvalue_2 (Class|BasicGruntCharacter|IsSameCamp "AllyActor"))
            (if (not _returnvalue_2)
              (goto _label))))))))

(event OnComponentEndOverlap(SphereDetection)
  (params (OverlappedComponent :type Primitive%20Component%20Object%20Reference) (OtherActor :type Actor%20Object%20Reference) (OtherComp :type Primitive%20Component%20Object%20Reference) (OtherBodyIndex :type Integer))
  (bind _spheredetection (Variables|Default|GetSphereDetection))
  (bind _overlappingactors (Collision|GetOverlappingActors _spheredetection 0 :!class /Script/Engine.PrimitiveComponent))
  (if (== OtherActor (Variables|Default|GetClosest%20Actor))
    (Variables|Default|SetClosest%20Actor (Variables|Default|GetNoneActor))
    (Default|CallOnNoEnemyDetected :!label _label)
    (elif (== (Utilities|Array|Length _overlappingactors) 0)
      (goto _label)
      (else
        (for _array_element _overlappingactors
          (bind _asbasic_grunt_character_bp (Utilities|Casting|CastToBasicGruntCharacter_BP _array_element)
            (:then
              (bind _returnvalue (Class|BasicGruntCharacter|IsSameCamp _asbasic_grunt_character_bp (Variables|Default|GetGruntCamp)))
              (if (not _returnvalue)
                (Utilities|IsValid (Variables|Default|GetClosest%20Actor) :!label _label_2
                  (:Is%20Valid
                    (if (> (Transformation|GetDistanceTo (Variables|Default|GetClosest%20Actor)) (Transformation|GetDistanceTo _array_element))
                      (Variables|Default|SetDistance%20ClosestActor (Transformation|GetDistanceTo (Variables|Default|GetClosest%20Actor)))
                      (Variables|Default|SetClosest%20Actor _array_element)
                      (Default|CallOnEnnemyDetected (Variables|Default|GetClosest%20Actor) (Variables|Default|GetDistance%20ClosestActor) :!label _label_3)
                      (else
                        (Variables|Default|SetDistance%20ClosestActor (Transformation|GetDistanceTo _array_element)))))
                  (:Is%20Not%20Valid
                    (Variables|Default|SetDistance%20ClosestActor (Transformation|GetDistanceTo _array_element))
                    (Variables|Default|SetClosest%20Actor _array_element)
                    (goto _label_3)))))
            (:CastFailed
              (Utilities|Casting|CastToRhuneProjectCharacter _array_element)
              (bind _returnvalue_2 (Class|BasicGruntCharacter|IsSameCamp "AllyActor"))
              (if (not _returnvalue_2)
                (goto _label_2)))))))))

(event EventBeginPlay
  (bind _mesh (Variables|Character|GetMesh))
  (bind _mesh_2 (Variables|Character|GetMesh))
  (bind _mesh_3 (Variables|Character|GetMesh))
  (bind _asgrunt_health_bar (Utilities|Casting|CastToGruntHealthBar (UserInterface|GetUserWidgetObject (Variables|Default|GetGruntHealthBar))))
  (Variables|/Game/Core/Grunt/GruntHealthBar.GruntHealthBar_C|SetGrunt _asgrunt_health_bar self)
  (Rendering|SetVisibility (Variables|Default|GetGruntHealthBar) false false)
  (bind _returnvalue (Class|BasicGruntCharacter|IsSameAuraType "Occulte"))
  (if _returnvalue
    (Rendering|Material|SetMaterial _mesh_2 1 "/Game/ModularRPGHeroesPolyart/Materials/Black.Black")
    (bind _returnvalue_2 (Class|BasicGruntCharacter|IsSameCamp "AllyActor"))
    (if _returnvalue_2
      (Rendering|Material|SetMaterial _mesh_3 0 "/Game/GruntMaterial/M_Dwarf_Grunt_ally_occulte.M_Dwarf_Grunt_ally_occulte")
      (else
        (Rendering|Material|SetMaterial _mesh_3 0 "/Game/GruntMaterial/M_Dwarf_Grunt_ennemy_occulte.M_Dwarf_Grunt_ennemy_occulte")))
    (Rendering|Material|SetMaterial _mesh_3 1 "/Game/GruntMaterial/Dwarf_Grunt_Equipment_occulte.Dwarf_Grunt_Equipment_occulte")
    (else
      (Rendering|Material|SetMaterial _mesh_2 1 "/Game/ModularRPGHeroesPolyart/Materials/White.White")
      (bind _returnvalue_3 (Class|BasicGruntCharacter|IsSameCamp "AllyActor"))
      (if _returnvalue_3
        (Rendering|Material|SetMaterial _mesh 0 "/Game/GruntMaterial/M_Dwarf_Grunt_ally_celeste.M_Dwarf_Grunt_ally_celeste")
        (else
          (Rendering|Material|SetMaterial _mesh 0 "/Game/GruntMaterial/M_Dwarf_Grunt_ennemy_celeste.M_Dwarf_Grunt_ennemy_celeste")))
      (Rendering|Material|SetMaterial _mesh 1 "/Game/GruntMaterial/Dwarf_Grunt_Equipment_celeste.Dwarf_Grunt_Equipment_celeste"))))

(event Collision|EventActorBeginOverlap
  (params (OtherActor :type Actor%20Object%20Reference)))

(event Game|Damage|EventAnyDamage
  (params (Damage :type Float%20%28single-precision%29) (DamageType :type Damage%20Type%20Object%20Reference) (InstigatedBy :type Controller%20Object%20Reference) (DamageCauser :type Actor%20Object%20Reference))
  (Class|BasicGruntCharacter|TakeDamages Damage DamageCauser))

(event EventTick
  (params (DeltaSeconds :type Float%20%28single-precision%29))
  (bind _grunthealthbar (Variables|Default|GetGruntHealthBar))
  (if (Variables|HpComponent|GetShowLifeBar)
    (if (<= (Transformation|GetDistanceTo (Game|GetPlayerCharacter 0)) (Variables|HpComponent|GetDistanceMaxShowHpBar))
      (Rendering|SetVisibility _grunthealthbar true false)
      (Transformation|SetWorldRotation (Variables|Default|GetGruntHealthBar) (Math|Rotator|FindLookatRotation (* (Transformation|GetActorLocation) "1.000000,1.000000, 0") (* (Transformation|GetActorLocation (Game|GetPlayerCameraManager 0)) "1.000000,1.000000, 0")) false false)
      (else
        (Rendering|SetVisibility _grunthealthbar false false)))))

(fn ConstructionScript)