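; Game manager Blueprint that drives the match flow from tutorial overlay through play to a win or lose screen.
; It shows the tutorial HUD at BeginPlay, then on Tick waits for IsGameStart before destroying all Wall actors and removing that HUD.
; Afterwards it polls IsLost, then IsWin, each tick; either result leads after a delay to its end-screen widget, disabled input and a paused game.
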(event EventBeginPlay
  (bind _returnvalue (UserInterface|CreateWidget "/Game/Core/UI/TutoHUD.TutoHUD_C"))
  (bind _output_get (Variables|Default|SetTutoHudReference _returnvalue))
  (UserInterface|Viewport|AddtoViewport _output_get 0))

(event Collision|EventActorBeginOverlap
  (params (OtherActor :type Actor%20Object%20Reference)))

(event EventTick
  (params (DeltaSeconds :type Float%20%28single-precision%29))
  (if (Variables|Default|GetStartFirstTick)
    (bind _returnvalue (Class|GameManager|IsLost))
    (if _returnvalue
      (Utilities|FlowControl|Delay 5.0)
      (bind _returnvalue_2 (UserInterface|CreateWidget "/Game/Core/UI/GameLostHUD.GameLostHUD_C"))
      (UserInterface|Viewport|AddtoViewport _returnvalue_2 0)
      (Input|DisableInput 0)
      (Game|SetGamePaused true)
      (else
        (bind _returnvalue_3 (Class|GameManager|IsWin))
        (if _returnvalue_3
          (Utilities|FlowControl|Delay 5.0)
          (bind _returnvalue_4 (UserInterface|CreateWidget "/Game/Core/UI/GameWinHUD.GameWinHUD_C"))
          (UserInterface|Viewport|AddtoViewport _returnvalue_4 0)
          (Input|DisableInput 0)
          (Game|SetGamePaused true))))
    (elif (Variables|Default|GetIsGameStart)
      (bind _outactors (Actor|GetAllActorsOfClass "/Game/Core/Wall.Wall_C"))
      (for _array_element _outactors
        (Actor|DestroyActor _array_element))
      (Variables|Default|SetStartFirstTick true)
      (Widget|RemovefromParent (Variables|Default|GetTutoHudReference)))))

(fn ConstructionScript)