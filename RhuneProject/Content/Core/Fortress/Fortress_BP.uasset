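; Capturable fortress actor that takes damage, can switch camps and shows its allegiance through its crystal material.
; A widget health bar is linked on BeginPlay, shown only when the player is near, and yawed toward the camera each Tick.
; AnyDamage calls TakeDamages, then on an IsSwitching flag re-checks the camp against AllyActor, swaps the material and shows a timed ally or enemy fortress-taken HUD.
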(event EventBeginPlay
  (bind _mesh (Variables|Character|GetMesh))
  (bind _asfortress_health_bar (Utilities|Casting|CastToFortressHealthBar (UserInterface|GetUserWidgetObject (Variables|Default|GetFortressHealthBar))))
  (Variables|/Game/Core/Fortress/FortressHealthBar.FortressHealthBar_C|SetFortress _asfortress_health_bar self)
  (bind _returnvalue (Class|Fortress|IsSameCamp "AllyActor"))
  (if _returnvalue
    (Rendering|Material|SetMaterial _mesh 1 "/Game/Core/Zoo/crystal.crystal")
    (else
      (Rendering|Material|SetMaterial _mesh 1 "/Game/Core/Zoo/crystale_rouge.crystale_rouge"))))

(event Collision|EventActorBeginOverlap
  (params (OtherActor :type Actor%20Object%20Reference)))

(event EventTick
  (params (DeltaSeconds :type Float%20%28single-precision%29))
  (bind _fortresshealthbar (Variables|Default|GetFortressHealthBar))
  (if (<= (Transformation|GetDistanceTo (Game|GetPlayerCharacter 0)) (Variables|HpComponent|GetDistanceMaxShowHpBar))
    (Rendering|SetVisibility _fortresshealthbar true false)
    (Transformation|SetWorldRotation (Variables|Default|GetFortressHealthBar) (Math|Rotator|FindLookatRotation (* (Transformation|GetActorLocation) "1.000000,1.000000,0.000000") (* (Transformation|GetActorLocation (Game|GetPlayerCameraManager 0)) "1.000000,1.000000,0.000000")) false false)
    (else
      (Rendering|SetVisibility _fortresshealthbar false false))))

(event Game|Damage|EventAnyDamage
  (params (Damage :type Float%20%28single-precision%29) (DamageType :type Damage%20Type%20Object%20Reference) (InstigatedBy :type Controller%20Object%20Reference) (DamageCauser :type Actor%20Object%20Reference))
  (bind _mesh (Variables|Character|GetMesh))
  (Class|Fortress|TakeDamages Damage)
  (if (Variables|Default|GetIsSwitching)
    (Variables|Default|SetIsSwitching false)
    (bind _returnvalue (Class|Fortress|IsSameCamp "AllyActor"))
    (if _returnvalue
      (Rendering|Material|SetMaterial _mesh 1 "/Game/Core/Zoo/crystal.crystal")
      (bind _returnvalue_2 (UserInterface|CreateWidget "/Game/Core/UI/EnemyFortressTakenHUD.EnemyFortressTakenHUD_C"))
      (UserInterface|Viewport|AddtoViewport _returnvalue_2 0)
      (Utilities|FlowControl|Delay 1e+01)
      (Widget|RemovefromParent _returnvalue_2)
      (else
        (Rendering|Material|SetMaterial _mesh 1 "/Game/Core/Zoo/crystale_rouge.crystale_rouge")
        (bind _returnvalue_3 (UserInterface|CreateWidget "/Game/Core/UI/AllyFortressTakenHUD.AllyFortressTakenHUD_C"))
        (UserInterface|Viewport|AddtoViewport _returnvalue_3 0)
        (Utilities|FlowControl|Delay 1e+01)
        (Widget|RemovefromParent _returnvalue_3)))))

(fn ConstructionScript)