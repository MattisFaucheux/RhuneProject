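; Player hero character with basic, laser and AoE attacks, a dash, aura switching, a map toggle and a death screen.
; Modular body parts follow the main mesh, and hair turns black or white with the aura type.
; ABP_Hero flags drive animations; its attack events toggle the hand hitbox, while delays time the special-attack hitboxes.
; Overlaps call DoDamages by attack type; incoming damage checks HpComponent for death.
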(event OnComponentBeginOverlap(HandCollision)
  (params (OverlappedComponent :type Primitive%20Component%20Object%20Reference) (OtherActor :type Actor%20Object%20Reference) (OtherComp :type Primitive%20Component%20Object%20Reference) (OtherBodyIndex :type Integer) (bFromSweep :type Boolean) (SweepResult :type Hit%20Result%20Structure%20%28by%20ref%29))
  (Class|RhuneProjectCharacter|DoDamages OtherActor "BasicAttack"))

(event OnComponentBeginOverlap(LaserCollision)
  (params (OverlappedComponent :type Primitive%20Component%20Object%20Reference) (OtherActor :type Actor%20Object%20Reference) (OtherComp :type Primitive%20Component%20Object%20Reference) (OtherBodyIndex :type Integer) (bFromSweep :type Boolean) (SweepResult :type Hit%20Result%20Structure%20%28by%20ref%29))
  (Class|RhuneProjectCharacter|DoDamages OtherActor "LaserAttack"))

(event OnComponentBeginOverlap(AoeCollision)
  (params (OverlappedComponent :type Primitive%20Component%20Object%20Reference) (OtherActor :type Actor%20Object%20Reference) (OtherComp :type Primitive%20Component%20Object%20Reference) (OtherBodyIndex :type Integer) (bFromSweep :type Boolean) (SweepResult :type Hit%20Result%20Structure%20%28by%20ref%29))
  (Class|RhuneProjectCharacter|DoDamages OtherActor "AoeAttack"))

(event Custom|OnAttackBeginEvent
  (Collision|SetCollisionEnabled (Variables|Default|GetHandCollision) "QueryOnly"))

(event Custom|OnAttackEndEvent
  (Collision|SetCollisionEnabled (Variables|Default|GetHandCollision) "NoCollision")
  (Variables|/Script/RhuneProject.HeroAnimInstance|SetIsAttacking (stale EventBeginPlay _asabp_hero) false)
  (Variables|Default|SetIsDoingAnAction false))

(event EventBeginPlay
  (bind _hair (Variables|Default|GetHair))
  (Class|SkinnedMeshComponent|SetMasterPoseComponent (Variables|Default|GetHair) (Variables|Character|GetMesh) false)
  (Class|RhuneProjectCharacter|SetAnimInstance)
  (bind _returnvalue (UserInterface|CreateWidget "/Game/Core/Hero/MainHUD.MainHUD_C"))
  (bind _output_get (Variables|Default|SetHUD%20Reference _returnvalue))
  (bind _returnvalue_2 (UserInterface|CreateWidget "/Game/Core/UI/MapHUD.MapHUD_C"))
  (bind _output_get_2 (Variables|Default|SetMapHudReference _returnvalue_2))
  (Variables|Default|SetIsMapActivate true)
  (UserInterface|Viewport|AddtoViewport _output_get 0)
  (Collision|SetCollisionEnabled (Variables|Default|GetLaserCollision) "NoCollision")
  (Collision|SetCollisionEnabled (Variables|Default|GetAoeCollision) "NoCollision")
  (Collision|SetCollisionEnabled (Variables|Default|GetHandCollision) "NoCollision")
  (bind _asabp_hero (Utilities|Casting|CastToABP_Hero (Components|SkeletalMesh|GetAnimInstance (Variables|Character|GetMesh))))
  (EventDispatchers|BindEventtoOnAttackBegin _asabp_hero (delegate Custom|OnAttackBeginEvent))
  (EventDispatchers|BindEventtoOnAttackEnd _asabp_hero (delegate Custom|OnAttackEndEvent))
  (bind _returnvalue_3 (Class|RhuneProjectCharacter|IsSameAuraType "Occulte"))
  (if _returnvalue_3
    (Rendering|Material|SetMaterial _hair 0 "/Game/ModularRPGHeroesPolyart/Materials/Black.Black")
    (else
      (Rendering|Material|SetMaterial _hair 0 "/Game/ModularRPGHeroesPolyart/Materials/White.White"))))

(event Game|Damage|EventAnyDamage
  (params (Damage :type Float%20%28single-precision%29) (DamageType :type Damage%20Type%20Object%20Reference) (InstigatedBy :type Controller%20Object%20Reference) (DamageCauser :type Actor%20Object%20Reference))
  (Class|RhuneProjectCharacter|TakeDamages Damage)
  (bind _returnvalue (Class|HpComponent|IsDead (Variables|Default|GetHpComponent)))
  (if _returnvalue
    (Input|DisableInput 0)
    (Utilities|FlowControl|Delay 5.0)
    (bind _returnvalue_2 (UserInterface|CreateWidget "/Game/Core/Hero/PlayerDeath.PlayerDeath_C"))
    (UserInterface|Viewport|AddtoViewport _returnvalue_2 0)))

(event Input|ActionEvents|InputActionSpecialAttack1
  (params (Key :type Key%20Structure :default "None"))
  (bind _lasercollision (Variables|Default|GetLaserCollision))
  (:Pressed
    (if (not (Variables|Default|GetIsDoingAnAction))
      (if (Variables|Default|GetCanDoLaserAttack)
        (Variables|Default|SetIsDoingAnAction true)
        (bind _asabp_hero (Utilities|Casting|CastToABP_Hero (Components|SkeletalMesh|GetAnimInstance (Variables|Character|GetMesh))))
        (Variables|/Script/RhuneProject.HeroAnimInstance|SetIsDoingBeamAttack _asabp_hero true)
        (Class|RhuneProjectCharacter|SetCantDoLaserAttack)
        (Utilities|FlowControl|Delay 0.8)
        (Collision|SetCollisionEnabled _lasercollision "QueryOnly")
        (Utilities|FlowControl|Delay 0.5)
        (Collision|SetCollisionEnabled _lasercollision "NoCollision")
        (Variables|Default|SetIsDoingAnAction false)
        (Class|RhuneProjectCharacter|CallLaserAttackReload)
        (Variables|/Script/RhuneProject.HeroAnimInstance|SetIsDoingBeamAttack _asabp_hero false)))))

(event Input|ActionEvents|InputActionF/TakeDamagess
  (params (Key :type Key%20Structure :default "None"))
  (:Pressed
    (Class|RhuneProjectCharacter|TakeDamages 5.0)
    (bind _returnvalue (Class|HpComponent|IsDead (Variables|Default|GetHpComponent)))
    (if _returnvalue
      (Input|DisableInput 0)
      (Utilities|FlowControl|Delay 5.0)
      (bind _returnvalue_2 (UserInterface|CreateWidget "/Game/Core/Hero/PlayerDeath.PlayerDeath_C"))
      (UserInterface|Viewport|AddtoViewport _returnvalue_2 0))))

(event Input|ActionEvents|InputActionSwitchAura
  (params (Key :type Key%20Structure :default "None"))
  (bind _hair (Variables|Default|GetHair))
  (:Pressed
    (bind _asabp_hero (Utilities|Casting|CastToABP_Hero (Components|SkeletalMesh|GetAnimInstance (Variables|Character|GetMesh))))
    (Variables|/Script/RhuneProject.HeroAnimInstance|SetIsDoingSwapAura _asabp_hero true)
    (Class|RhuneProjectCharacter|SwitchAura)
    (bind _returnvalue (Class|RhuneProjectCharacter|IsSameAuraType "Occulte"))
    (if _returnvalue
      (Rendering|Material|SetMaterial _hair 0 "/Game/ModularRPGHeroesPolyart/Materials/Black.Black")
      (else
        (Rendering|Material|SetMaterial _hair 0 "/Game/ModularRPGHeroesPolyart/Materials/White.White")))
    (Utilities|FlowControl|Delay 0.8)
    (Variables|/Script/RhuneProject.HeroAnimInstance|SetIsDoingSwapAura _asabp_hero false)))

(event Input|ActionEvents|InputActionSpecialAttack2
  (params (Key :type Key%20Structure :default "None"))
  (bind _aoecollision (Variables|Default|GetAoeCollision))
  (:Pressed
    (if (not (Variables|Default|GetIsDoingAnAction))
      (if (Variables|Default|GetCanDoAoeAttack)
        (Variables|Default|SetIsDoingAnAction true)
        (bind _asabp_hero (Utilities|Casting|CastToABP_Hero (Components|SkeletalMesh|GetAnimInstance (Variables|Character|GetMesh))))
        (Variables|/Script/RhuneProject.HeroAnimInstance|SetIsDoingAoeAttack _asabp_hero true)
        (Class|RhuneProjectCharacter|SetCantDoAoeAttack)
        (Utilities|FlowControl|Delay 0.4)
        (Collision|SetCollisionEnabled _aoecollision "QueryOnly")
        (Utilities|FlowControl|Delay 0.5)
        (Collision|SetCollisionEnabled _aoecollision "NoCollision")
        (Variables|Default|SetIsDoingAnAction false)
        (Class|RhuneProjectCharacter|CallAoeAttackReload)
        (Variables|/Script/RhuneProject.HeroAnimInstance|SetIsDoingAoeAttack _asabp_hero false)))))

(event Input|ActionEvents|InputActionToggleMap
  (params (Key :type Key%20Structure :default "None"))
  (bind _maphudreference (Variables|Default|GetMapHudReference))
  (:Pressed
    (if (Variables|Default|GetIsMapActivate)
      (Widget|RemovefromParent _maphudreference)
      (Variables|Default|SetIsMapActivate false)
      (else
        (UserInterface|Viewport|AddtoViewport _maphudreference 0)
        (Variables|Default|SetIsMapActivate true)))))

(fn ConstructionScript)

(fn DoDash
  (if (AI|Components|NavMovement|IsMovingonGround (Variables|Character|GetCharacterMovement))
    (Character|LaunchCharacter (* (Math|Vector|GetForwardVector (Variables|Default|GetCapsuleComponent)) 1e+04) false false)
    (bind _asabp_hero (Utilities|Casting|CastToABP_Hero (Components|SkeletalMesh|GetAnimInstance (Variables|Character|GetMesh))))
    (Variables|/Script/RhuneProject.HeroAnimInstance|SetIsDashing _asabp_hero true)))